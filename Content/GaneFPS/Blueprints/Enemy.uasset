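; Enemy Blueprint with a health bar widget, contact attack and configurable body color.
; On BeginPlay it snaps a sphere to the mesh's CollisionSocket and initializes the widget, while hitting a HeRoCharacter calls that character's AttackHero.
; The Attack event damages this enemy by a fixed amount, updates the bar and destroys it at zero health.
; Playanim plays a jump montage, and the construction script tints the mesh through a dynamic material.
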(event `self.ReceiveTick`
  (params (DeltaSeconds :type "Float (single-precision)")))

(event `self.ReceiveBeginPlay`
  (`SceneComponent.K2_AttachToComponent` (`self.Sphere`) (`self.Mesh`) "CollisionSocket" "SnapToTarget" "KeepWorld" "KeepRelative" true)
  (bind _aswg_health_enemy (cast `/Game/UI/WG_HealthEnemy` (`WidgetComponent.GetUserWidgetObject` (`self.Health`))))
  (set `/Game/UI/WG_HealthEnemy.CurrentHealth` 100.0 _aswg_health_enemy)
  (set `/Game/UI/WG_HealthEnemy.TotalHealth` 100.0 _aswg_health_enemy))

(event `self.ReceiveHit`
  (params (MyComp :type "PrimitiveComponent Object Reference") (Other :type "Actor Object Reference") (OtherComp :type "PrimitiveComponent Object Reference") (bSelfMoved :type Boolean) (HitLocation :type "Vector Structure") (HitNormal :type "Vector Structure") (NormalImpulse :type "Vector Structure") (Hit :type "HitResult Structure (by ref)"))
  (bind _ashe_ro_character (cast `/Game/GaneFPS/Blueprints/HeRoCharacter` Other))
  (`/Game/GaneFPS/Blueprints/HeRoCharacter.AttackHero` _ashe_ro_character))

(event `Attack`
  (bind _output_get (set `self.HealthEnemy` (- (`self.HealthEnemy`) 30.0)))
  (bind _aswg_health_enemy (cast `/Game/UI/WG_HealthEnemy` (`WidgetComponent.GetUserWidgetObject` (`self.Health`))))
  (set `/Game/UI/WG_HealthEnemy.CurrentHealth` _output_get _aswg_health_enemy)
  (if (<= (`self.HealthEnemy`) 0.0)
    (`self.K2_DestroyActor`)))

(event `Playanim`
  ;[1 1 1] AnemyAttack
  (`|PlayMontage` (`self.Mesh`) "/Game/Mannequin/Animations/ThirdPerson_Jump_Montage.ThirdPerson_Jump_Montage"))

(fn `UserConstructionScript`
  (bind _returnvalue (`PrimitiveComponent.CreateDynamicMaterialInstance` (`self.Mesh`) 0 null "None"))
  (bind _output_get (set `self.DynaMat` _returnvalue))
  (`MaterialInstanceDynamic.SetVectorParameterValue` _output_get "BodyColor" (`self.Color`)))