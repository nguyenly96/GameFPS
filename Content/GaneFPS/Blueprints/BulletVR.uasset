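; BulletVR is a VR bullet actor that reacts on Hit to whatever it strikes.
; For an Enemy it calls Attack, then, if the enemy is still valid, spawns a fire particle at its location and destroys itself.
; Other hits spawn the same effect at the hit location and destroy the bullet.
; A second Sequence branch then calls HealthEnemy when the hit actor is an EnemyVR.
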(event `self.ReceiveHit`
  (params (MyComp :type "PrimitiveComponent Object Reference") (Other :type "Actor Object Reference") (OtherComp :type "PrimitiveComponent Object Reference") (bSelfMoved :type Boolean) (HitLocation :type "Vector Structure") (HitNormal :type "Vector Structure") (NormalImpulse :type "Vector Structure") (Hit :type "HitResult Structure (by ref)"))
  (`|ExecutionSequence`
    (:`then_0`
      (bind _asenemy (cast `/Game/GaneFPS/Blueprints/Enemy` Other)
        (:`then`
          (`/Game/GaneFPS/Blueprints/Enemy.Attack` _asenemy)
          (`/Engine/EditorBlueprintResources/StandardMacros.IsValid` _asenemy
            (:`Is Valid`
              (`GameplayStatics.SpawnEmitterAtLocation` "/Game/StarterContent/Particles/P_Fire1.P_Fire1" (`self.K2_GetActorLocation` _asenemy))
              (`self.K2_DestroyActor`))))
        (:`CastFailed`
          (`GameplayStatics.SpawnEmitterAtLocation` "/Game/StarterContent/Particles/P_Fire1.P_Fire1" HitLocation)
          (`self.K2_DestroyActor`))))
    (:`then_1`
      (bind _asenemy_vr (cast `/Game/GameVR/AIEnemy/EnemyVR` Other))
      (`/Game/GameVR/AIEnemy/EnemyVR.HealthEnemy` _asenemy_vr))))

(fn `UserConstructionScript`)