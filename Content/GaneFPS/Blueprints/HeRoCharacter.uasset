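; HeRoCharacter is a player character Blueprint with movement, jumping, weapon attacks and health.
; Axis inputs drive control-rotation-relative movement, pitch/yaw look and a stick-style look that sets control rotation directly, while the Shift axis event sets walk speed.
; BeginPlay spawns a weapon, attaches it to a mesh socket and adds a health widget to the viewport.
; Fire calls the weapon's Attack, and AttackHero subtracts health, destroying the actor at zero.
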(event `InputAxis|Shift`
  (params (AxisValue :type "Float (single-precision)"))
  (set `CharacterMovementComponent.MaxWalkSpeed` 1000.0 (`self.CharacterMovement`)))

(event `InputAxis|MoveForWord`
  (params (AxisValue :type "Float (single-precision)"))
  (`self.AddMovementInput` (`KismetMathLibrary.GetForwardVector` (`self.GetControlRotation`)) AxisValue))

(event `InputAxis|MoveRight`
  (params (AxisValue :type "Float (single-precision)"))
  (`self.AddMovementInput` (`KismetMathLibrary.GetRightVector` (`self.GetControlRotation`)) AxisValue))

(event `InputAxis|LookUp`
  (params (AxisValue :type "Float (single-precision)"))
  (bind _returnvalue (`KismetMathLibrary.MakeVector` AxisValue (stale `InputAxis|LookRight` AxisValue)))
  (if (> (`KismetMathLibrary.VSize` _returnvalue) 0.25) :!label _label
    (`Controller.SetControlRotation` (`self.GetController`) (`KismetMathLibrary.Conv_VectorToRotator` _returnvalue))))

(event `InputAxis|LookRight`
  (params (AxisValue :type "Float (single-precision)"))
  (goto _label))

(event `InputAction|Jump`
  (params (Key :type "Key Structure"))
  (:`Pressed`
    (`self.Jump`)))

(event `InputAxis|Lookup1`
  (params (AxisValue :type "Float (single-precision)"))
  (`self.AddControllerPitchInput` AxisValue))

(event `InputAxis|Turn1`
  (params (AxisValue :type "Float (single-precision)"))
  (`self.AddControllerYawInput` AxisValue))

(event `self.ReceiveBeginPlay`
  (bind _mesh (`self.Mesh`))
  (bind _returnvalue (`|SpawnActorFromClass` "/Game/GaneFPS/Blueprints/WeaPon.WeaPon_C" (`KismetMathLibrary.Conv_VectorToTransform` (`SceneComponent.K2_GetComponentLocation` _mesh)) "Undefined" "OverrideRootScale" null null))
  (bind _output_get (set `self.Weapon` _returnvalue))
  (`self.K2_AttachToComponent` _output_get _mesh "WeaponSoeeecket" "SnapToTarget" "KeepWorld" "KeepRelative" true)
  (bind _returnvalue_2 (`|CreateWidget` "/Game/UI/WG_Health1.WG_Health1_C"))
  (`UserWidget.AddToViewport` _returnvalue_2 0))

(event `InputAction|Fire`
  (params (Key :type "Key Structure"))
  (:`Pressed`
    (`/Game/GaneFPS/Blueprints/WeaPon.Attack` (`self.Weapon`))))

(event `AttackHero`
  (set `self.Health` (- (`self.Health`) 5.0))
  (if (<= (`self.Health`) 0.0)
    (`self.K2_DestroyActor`)))

(fn `UserConstructionScript`)